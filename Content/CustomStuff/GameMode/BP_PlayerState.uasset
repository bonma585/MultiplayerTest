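; BP_PlayerState handles respawning for two BP_Ghost players and refreshes the score on the HUD.
; Tick polls the ghosts at player indices 1 and 3, checking the second only while the first is not Dead.
; A Dead ghost drops its flag, is hidden with input disabled, teleports to a fixed point after a delay, then returns as Alive.
; BeginPlay and SetScore both call UpdateScore on WBPHUD.
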(event Custom|SetScore
  ;[1 1 1] Set Scores in WBP_HUD
  (Default|UpdateScore (Variables|Default|GetWBP_HUD)))

(event EventTick
  (params (DeltaSeconds :type Float%20%28single-precision%29))
  (bind _asbp_ghost (Utilities|Casting|CastToBP_Ghost (Game|GetPlayerCharacter 1)))
  (bind _asbp_ghost_2 (Utilities|Casting|CastToBP_Ghost (Game|GetPlayerCharacter 3))
    (:then
      _)
    (:CastFailed
      _))
  (switch Utilities|FlowControl|Switch|SwitchonE_PlayerState (Variables|/Game/TopDown/Blueprints/BP_Ghost.BP_Ghost_C|GetState _asbp_ghost)
    (:NewEnumerator0
      (switch Utilities|FlowControl|Switch|SwitchonE_PlayerState (Variables|/Game/TopDown/Blueprints/BP_Ghost.BP_Ghost_C|GetState _asbp_ghost_2) :!label _label
        (:NewEnumerator2
          (switch Utilities|FlowControl|Switch|SwitchonE_PlayerState "NewEnumerator1"
            (:NewEnumerator1
              (Development|PrintString "Respawning")
              (Variables|/Game/TopDown/Blueprints/BP_Ghost.BP_Ghost_C|SetbHasFlag _asbp_ghost_2 false)
              (Rendering|SetVisibility (Variables|/Game/TopDown/Blueprints/BP_Ghost.BP_Ghost_C|Getsm_ghost _asbp_ghost_2) false false)
              (Input|DisableInput _asbp_ghost_2 0)
              (Utilities|FlowControl|Delay 1.5)
              (Transformation|Teleport _asbp_ghost_2 "-11200.000000,3300.000000,100.000000" "0, 0, 0")
              (Utilities|FlowControl|Delay 0.75)
              (Rendering|SetVisibility (Variables|/Game/TopDown/Blueprints/BP_Ghost.BP_Ghost_C|Getsm_ghost _asbp_ghost_2) true false)
              (Input|EnableInput _asbp_ghost_2 0)
              (Variables|/Game/TopDown/Blueprints/BP_Ghost.BP_Ghost_C|SetState _asbp_ghost_2 "NewEnumerator0"))))))
    (:NewEnumerator1
      (goto _label))
    (:NewEnumerator2
      (switch Utilities|FlowControl|Switch|SwitchonE_PlayerState "NewEnumerator1"
        (:NewEnumerator1
          (Development|PrintString "Respawning")
          (Variables|/Game/TopDown/Blueprints/BP_Ghost.BP_Ghost_C|SetbHasFlag _asbp_ghost false)
          (Rendering|SetVisibility (Variables|/Game/TopDown/Blueprints/BP_Ghost.BP_Ghost_C|Getsm_ghost _asbp_ghost) false false)
          (Input|DisableInput _asbp_ghost 0)
          (Utilities|FlowControl|Delay 1.5)
          (Transformation|Teleport _asbp_ghost "-11200.000000,3300.000000,100.000000" "0, 0, 0")
          (Utilities|FlowControl|Delay 0.75)
          (Rendering|SetVisibility (Variables|/Game/TopDown/Blueprints/BP_Ghost.BP_Ghost_C|Getsm_ghost _asbp_ghost) true false)
          (Input|EnableInput _asbp_ghost 0)
          (Variables|/Game/TopDown/Blueprints/BP_Ghost.BP_Ghost_C|SetState _asbp_ghost "NewEnumerator0"))))))

(event EventBeginPlay
  ;[1 1 1] Set Scores in WBP_HUD
  (Default|UpdateScore (Variables|Default|GetWBP_HUD)))

(fn ConstructionScript)