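; Multiplayer game mode that splits joining players into Ghost and Hunter sides.
; On PostLogin, a running player index sends the first and third players to the ghost team and all others to the hunter team.
; Each player gets a team value on BP_PlayerState, looked up by that index rather than from the new controller.
; It then spawns BP_Ghost or BP_Hunter at that side's fixed location and has the controller possess it.
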(event EventPostLogin
  (params (NewPlayer :type Player%20Controller%20Object%20Reference))
  ;[1 1 1] Set Teams
  (bind _asbp_player_state (Utilities|Casting|CastToBP_PlayerState (Game|GetPlayerState (Variables|Default|GetPlayerIndex))))
  (if (== (Variables|Default|GetPlayerIndex) 0)
    (Variables|Default|SetPlayerIndex (+ (Variables|Default|GetPlayerIndex) 1) :!label _label)
    (Variables|/Game/CustomStuff/GameMode/BP_PlayerState.BP_PlayerState_C|SetTeam _asbp_player_state "NewEnumerator0")
    (bind _returnvalue (Game|SpawnActorfromClass "/Game/TopDown/Blueprints/BP_Ghost.BP_Ghost_C" (Math|Transform|MakeTransform "-11200.000000,3300.000000,100.000000") "Undefined" "MultiplyWithRoot" 0 0))
    (Pawn|Possess NewPlayer _returnvalue)
    (elif (== (Variables|Default|GetPlayerIndex) 2)
      (goto _label)
      (else
        (Variables|Default|SetPlayerIndex (+ (Variables|Default|GetPlayerIndex) 1))
        (Variables|/Game/CustomStuff/GameMode/BP_PlayerState.BP_PlayerState_C|SetTeam _asbp_player_state "NewEnumerator1")
        (bind _returnvalue_2 (Game|SpawnActorfromClass "/Game/TopDown/Blueprints/BP_Hunter.BP_Hunter_C" (Math|Transform|MakeTransform "-9300.000000,920.000000,100.000000") "Undefined" "MultiplyWithRoot" 0 0))
        (Pawn|Possess NewPlayer _returnvalue_2)))))

(fn ConstructionScript)